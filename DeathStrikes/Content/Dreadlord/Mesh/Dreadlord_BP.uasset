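; Dreadlord boss enemy character with a widget health bar that shows while the Knight is inside its activator radius.
; AnyDamage lowers Health and refreshes the bar; at zero it ragdolls, stops AI logic, drops its damage collider, then pauses on a victory screen.
; Overlapping the damage collider directly reduces the Knight's health, and a custom event plays the attack montage.
; Click-to-target logic and an ApplyDamage call are left unwired.
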(event OnComponentBeginOverlap(DamagePlayerCollider)
  (params (OverlappedComponent :type Primitive%20Component%20Object%20Reference) (OtherActor :type Actor%20Object%20Reference) (OtherComp :type Primitive%20Component%20Object%20Reference) (OtherBodyIndex :type Integer) (bFromSweep :type Boolean) (SweepResult :type Hit%20Result%20Structure%20%28by%20ref%29))
  ;[0.4948 0.03951 0.04115] ENEMY HEALTH & Linking to Widget
  ;;[1 1 1] Enemy Collider that DAMAGES PLAYER HEALTH
  (bind _asknight (Utilities|Casting|CastToKnight OtherActor))
  (Variables|/Game/ThirdPersonBP/Blueprints/Knight.Knight_C|SetKhightHealth _asknight (- (Variables|/Game/ThirdPersonBP/Blueprints/Knight.Knight_C|GetKhightHealth _asknight) 0.1)))

(event OnComponentBeginOverlap(BossHealthRadiusActivator)
  (params (OverlappedComponent :type Primitive%20Component%20Object%20Reference) (OtherActor :type Actor%20Object%20Reference) (OtherComp :type Primitive%20Component%20Object%20Reference) (OtherBodyIndex :type Integer) (bFromSweep :type Boolean) (SweepResult :type Hit%20Result%20Structure%20%28by%20ref%29))
  ;[0.4948 0.03951 0.04115] ENEMY HEALTH & Linking to Widget
  ;;[1 1 1] Health Radius Activator
  (Utilities|Casting|CastToKnight OtherActor)
  (Rendering|SetVisibility (Variables|Default|GetBossHealthBar) true false))

(event OnComponentEndOverlap(BossHealthRadiusActivator)
  (params (OverlappedComponent :type Primitive%20Component%20Object%20Reference) (OtherActor :type Actor%20Object%20Reference) (OtherComp :type Primitive%20Component%20Object%20Reference) (OtherBodyIndex :type Integer))
  ;[0.4948 0.03951 0.04115] ENEMY HEALTH & Linking to Widget
  ;;[1 1 1] Health Radius Activator
  (Utilities|Casting|CastToKnight OtherActor)
  (Rendering|SetVisibility (Variables|Default|GetBossHealthBar) false false))

(event Custom|ClearTarget
  ;[1 1 1] Detects player click and sets variable "Target" to Self
  (Rendering|SetVisibility (Variables|Default|GetTargetIndicator) false false))

(event Custom|CustomEvent
  (Animation|PlayAnimMontage "/Game/JC_TEMP/Animation/AttackRunAI.AttackRunAI" 1.0 "None"))

(event EventBeginPlay
  ;[0.4948 0.03951 0.04115] ENEMY HEALTH & Linking to Widget
  (bind _asbp_boss_health (Utilities|Casting|CastTobp_BossHealth (UserInterface|GetUserWidgetObject (Variables|Default|GetBossHealthBar))))
  (bind _output_get (Variables|Default|SetBossHealthBarWidget _asbp_boss_health))
  (Variables|/Game/UserInterface/In-GameWidgets/bp_BossHealth.bp_BossHealth_C|SetBossNPC _output_get 0)
  (Default|UpdateHealth _output_get))

(event Collision|EventHit
  (params (MyComp :type Primitive%20Component%20Object%20Reference) (Other :type Actor%20Object%20Reference) (OtherComp :type Primitive%20Component%20Object%20Reference) (bSelfMoved :type Boolean) (HitLocation :type Vector :default "0, 0, 0") (HitNormal :type Vector :default "0, 0, 0") (NormalImpulse :type Vector :default "0, 0, 0") (Hit :type Hit%20Result%20Structure%20%28by%20ref%29)))

(event MouseInput|EventActorOnClicked
  (params (ButtonPressed :type Key%20Structure :default "None"))
  ;[1 1 1] Detects player click and sets variable "Target" to Self
  (bind _asmy_controller (Utilities|Casting|CastToMyController (Game|GetPlayerController 0))))

(event Game|Damage|EventAnyDamage
  (params (Damage :type Float%20%28single-precision%29) (DamageType :type Damage%20Type%20Object%20Reference) (InstigatedBy :type Controller%20Object%20Reference) (DamageCauser :type Actor%20Object%20Reference))
  ;[0.4948 0.03951 0.04115] ENEMY HEALTH & Linking to Widget
  ;;[1 1 1] Once Enemy Health is <= 0 Health bar gets destroyed and ragdoll physics take over
  (bind _output_get (Variables|Default|SetHealth (- (Variables|Default|GetHealth) Damage)))
  (Utilities|FlowControl|Sequence
    (:then_0
      (Default|UpdateHealth (Variables|Default|GetBossHealthBarWidget)))
    (:then_1
      (if (<= _output_get 0.0)
        (Components|DestroyComponent (Variables|Collision|GetCapsuleComponent))
        (Physics|SetSimulatePhysics (Variables|Character|GetMesh) true)
        ;;[1 1 1] Enemy loses 100% functionality
        (AI|Logic|StopLogic (Variables|/Script/AIModule.AIController|GetBrainComponent (AI|GetAIController self)) "")
        ;;[1 1 1] Destroys player dmg collider on death
        (Components|DestroyComponent (Variables|Default|GetDamage%20Player%20Collider))
        ;;[1 1 1] Victory Widget when you kill the boss
        (Utilities|FlowControl|Delay 2.0)
        (bind _returnvalue (UserInterface|CreateWidget "/Game/UserInterface/In-GameWidgets/Victory_Widget.Victory_Widget_C"))
        (UserInterface|Viewport|AddtoViewport _returnvalue 0)
        (Variables|/Script/Engine.PlayerController|SetbShowMouseCursor (Game|GetPlayerController 0) true)
        (Game|SetGamePaused true)))))

(fn ConstructionScript)